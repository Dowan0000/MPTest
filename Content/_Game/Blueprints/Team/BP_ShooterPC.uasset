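; Shooter player controller that handles team selection and the spawn request that follows it.
; CreateTeamWidget shows WBP_TeamWidget, switches input to Game and UI, and reveals the mouse cursor.
; TeamSelect runs only with authority, passing the chosen team and this controller to BP_TeamGameMode's ReqSpawn.
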(event Custom|TeamSelect
  (params (Team :type ETeam%20Enum :default "ET_NoTeam"))
  (Networking|SwitchHasAuthority
    (:Authority
      (bind _asbp_team_game_mode (Utilities|Casting|CastToBP_TeamGameMode (Game|GetGameMode)))
      (Default|ReqSpawn _asbp_team_game_mode Team self))))

(event EventBeginPlay)

(event EventTick
  (params (DeltaSeconds :type Float%20%28single-precision%29)))

(event EventCreateTeamWidget
  (bind _returnvalue (UserInterface|CreateWidget "/Game/_Game/Blueprints/Team/WBP_TeamWidget.WBP_TeamWidget_C"))
  (UserInterface|Viewport|AddtoViewport _returnvalue 0)
  (Input|SetInputModeGameandUI self 0 "DoNotLock" true)
  (Variables|Default|SetbShowMouseCursor true))

(fn ConstructionScript)