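; Team game mode that spawns and possesses a red or blue shooter character for a player controller.
; ReqSpawn switches on the requested team and picks a random StartRed or StartBlue actor in the level as the spawn transform.
; It spawns that team's character class, adjusting for collision but always spawning, then has the controller possess it.
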(event Custom|ReqSpawn
  (params (Team :type ETeam%20Enum :default "ET_NoTeam") (PC :type BP%20Shooter%20PC%20Object%20Reference))
  (switch Utilities|FlowControl|Switch|SwitchonETeam Team
    (:ET_RedTeam
      (bind _outactors (Actor|GetAllActorsOfClass "/Game/_Game/Blueprints/Team/StartRed.StartRed_C"))
      (bind _returnvalue (Game|SpawnActorfromClass "/Game/_Game/Blueprints/Team/BP_ShooterCharacterRed.BP_ShooterCharacterRed_C" (Transformation|GetActorTransform (Utilities|Array|Get(acopy) _outactors (Math|Random|RandomInteger (Utilities|Array|Length _outactors)))) "AdjustIfPossibleButAlwaysSpawn" 0 0))
      (Pawn|Possess PC _returnvalue))
    (:ET_BlueTeam
      (bind _outactors_2 (Actor|GetAllActorsOfClass "/Game/_Game/Blueprints/Team/StartBlue.StartBlue_C"))
      (bind _returnvalue_2 (Game|SpawnActorfromClass "/Game/_Game/Blueprints/Team/BP_ShooterCharacterBlue.BP_ShooterCharacterBlue_C" (Transformation|GetActorTransform (Utilities|Array|Get(acopy) _outactors_2 (Math|Random|RandomInteger (Utilities|Array|Length _outactors_2)))) "AdjustIfPossibleButAlwaysSpawn" 0 0))
      (Pawn|Possess PC _returnvalue_2))))

(event EventBeginPlay)

(event EventTick
  (params (DeltaSeconds :type Float%20%28single-precision%29)))

(fn ConstructionScript)